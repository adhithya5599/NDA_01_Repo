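; BP_Hide is an interactable hiding spot that moves the player character into and out of hiding.
; StartInteract starts a looping timer at the frame's delta time, sliding the player at constant speed to PlayerPosition or ExitPosition, depending on IsHiding.
; Entering disables collision and movement before the slide.
; On arrival the timers are cleared and IsHiding flips, with collision and walking restored on exit.
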(event Custom|MoveCharacter
  (bind _playerref (Variables|Default|GetPlayerRef))
  (Transformation|SetActorTransform _playerref (Math|Transform|MakeTransform (Math|Interpolation|VInterptoConstant (Transformation|GetActorLocation _playerref) (Transformation|GetWorldLocation (select (Variables|/Game/FirstPerson/Blueprints/BP_FirstPersonCharacter.BP_FirstPersonCharacter_C|GetisHiding (Variables|Default|GetPlayerRef)) (Variables|Default|GetExitPosition) (Variables|Default|GetPlayerPosition))) (Utilities|Time|GetWorldDeltaSeconds) 1e+03) "0, 0, 0" "1.000000,1.000000,1.000000"))
  (if (Utilities|Operators|EqualEqual (Transformation|GetActorLocation (Variables|Default|GetPlayerRef)) (Transformation|GetWorldLocation (select (Variables|/Game/FirstPerson/Blueprints/BP_FirstPersonCharacter.BP_FirstPersonCharacter_C|GetisHiding (Variables|Default|GetPlayerRef)) (Variables|Default|GetExitPosition) (Variables|Default|GetPlayerPosition))) 0.01)
    (Utilities|Time|ClearandInvalidateTimerbyHandle (stale EventStartInteract _returnvalue_2))
    (Utilities|Time|ClearandInvalidateTimerbyHandle (stale EventStartInteract _returnvalue))
    (CallFunction|FinishedHidding)))

(event Custom|FinishedHidding
  (bind _playerref (Variables|Default|GetPlayerRef))
  (if (Variables|/Game/FirstPerson/Blueprints/BP_FirstPersonCharacter.BP_FirstPersonCharacter_C|GetisHiding _playerref)
    (Variables|/Game/FirstPerson/Blueprints/BP_FirstPersonCharacter.BP_FirstPersonCharacter_C|SetisHiding _playerref false)
    (Collision|SetActorEnableCollision _playerref true)
    (Pawn|Components|CharacterMovement|SetMovementMode (Variables|/Script/Engine.Character|GetCharacterMovement _playerref) "MOVE_Walking" 0)
    (else
      (Variables|/Game/FirstPerson/Blueprints/BP_FirstPersonCharacter.BP_FirstPersonCharacter_C|SetisHiding _playerref true))))

(event EventStartInteract
  (bind _playerref (Variables|Default|GetPlayerRef))
  (if (Variables|/Game/FirstPerson/Blueprints/BP_FirstPersonCharacter.BP_FirstPersonCharacter_C|GetisHiding (Variables|Default|GetPlayerRef))
    (bind _returnvalue (Utilities|Time|SetTimerbyEvent (delegate Custom|MoveCharacter) (Utilities|Time|GetWorldDeltaSeconds) true))
    (else
      (Collision|SetActorEnableCollision _playerref false)
      (Pawn|Components|CharacterMovement|DisableMovement (Variables|/Script/Engine.Character|GetCharacterMovement _playerref))
      (bind _returnvalue_2 (Utilities|Time|SetTimerbyEvent (delegate Custom|MoveCharacter) (Utilities|Time|GetWorldDeltaSeconds) true)))))

(event EventBeginPlay
  (bind _asbp_first_person_character (Utilities|Casting|CastToBP_FirstPersonCharacter (Game|GetPlayerCharacter 0)))
  (Variables|Default|SetPlayerRef _asbp_first_person_character))

(fn ConstructionScript)