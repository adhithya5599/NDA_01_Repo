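; BP_DoorCode is an interactable actor that shows a keypad UI for a code-locked door.
; StartInteract shows the cursor, switches to UI-only input and creates WBP_KeyPad, passing itself as a reference.
; Tick polls CanOpenDoor and, through a DoOnce, removes the keypad and restores game-only input with a hidden cursor.
; This graph neither sets that flag nor moves a door.
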(event EventBeginPlay)

(event Collision|EventActorBeginOverlap
  (params (OtherActor :type Actor%20Object%20Reference)))

(event EventTick
  (params (DeltaSeconds :type Float%20%28single-precision%29))
  (bind _returnvalue (Game|GetPlayerController 0))
  (if (Variables|Default|GetcanOpenDoor)
    (Utilities|FlowControl|DoOnce false
      (:Completed
        (Widget|RemovefromParent (stale EventStartInteract _returnvalue_2))
        (Variables|/Script/Engine.PlayerController|SetbShowMouseCursor _returnvalue false)
        (Input|SetInputModeGameOnly _returnvalue false)))))

(event EventStartInteract
  (bind _returnvalue (Game|GetPlayerController 0))
  (Variables|/Script/Engine.PlayerController|SetbShowMouseCursor _returnvalue true)
  (Input|SetInputModeUIOnly _returnvalue 0 "DoNotLock" false)
  (bind _returnvalue_2 (UserInterface|CreateWidget "/Game/NDA/UI/WBP_KeyPad.WBP_KeyPad_C" 0 self))
  (UserInterface|Viewport|AddtoViewport _returnvalue_2 0))

(fn ConstructionScript)